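; Monster enemy that roams randomly until it sees the player or survives a bullet hit, then chases.
; A looping AIMoveTo drives both states, returning to roaming when the chase fails.
; On reaching the player it stops and briefly enables overlap events on its attack area to deal damage.
; Bullet overlaps reduce health; death ragdolls the mesh, increments the game mode's kill count and destroys the actor.
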(event `self.感測元件.OnSeePawn`
  (params (Pawn :type "Pawn Object Reference"))
  (bind _charactermovement (`self.CharacterMovement`))
  (bind `_攻擊區域` (`self.攻擊區域`))
  ;[0.2889 1 0.3106] 看到玩家保存玩家資訊
  (bind `_asbp_玩家控制` (cast `/Game/BP/BP_玩家控制` Pawn))
  (set `self.玩家控制` `_asbp_玩家控制`)
  (set `self.是否看到玩家` true :!label _label)
  (set `self.停留時間` 0.0) ; 看到玩家後馬上跟蹤玩家
  (`/Engine/EditorBlueprintResources/StandardMacros.DoOnce` false
    (:`Completed`
      ;[1 1 1] 判斷有沒有看到玩家
      (if (`self.是否看到玩家`) :!label _label_2
        ;[1 0.3521 0.1511] 看到玩家後 : 追蹤玩家
        (`|AIMoveTo` self (0.0 0.0 0.0) (`self.玩家控制`) (`self.停止半徑`)
          (:`OnSuccess`
            ;[0.9164 0.2395 1] 攻擊狀態
            (set `self.攻擊` true)
            (set `CharacterMovementComponent.MaxWalkSpeed` 0.0 _charactermovement)
            (`KismetSystemLibrary.Delay` 1.0)
            (set `PrimitiveComponent.bGenerateOverlapEvents` true `_攻擊區域`)
            (`KismetSystemLibrary.Delay` 0.4) ; 手舉起來時間
            (set `PrimitiveComponent.bGenerateOverlapEvents` false `_攻擊區域`)
            (`KismetSystemLibrary.Delay` 1.2) ; 怪物下手攻擊
            (set `CharacterMovementComponent.MaxWalkSpeed` 500.0 _charactermovement)
            (set `self.攻擊` false)
            (goto _label_2))
          (:`OnFail`
            (set `self.是否看到玩家` false)
            (set `self.停留時間` 3.0) ; 恢復停留最大值為3
            (goto _label_2)))
        (else
          ;[1 0.3471 0.1257] 沒看到玩家 : 隨機走動
          (`|AIMoveTo` self (`NavigationSystemV1.K2_GetRandomReachablePointInRadius` (`SceneComponent.K2_GetComponentLocation` (`self.CapsuleComponent`)) (`self.隨機走動半徑`) null null) null (`self.停止半徑`) ; AI移動節點:移動到指定座標
            (:`then`
              ;;[1 1 1] 隨機停留
              (`KismetSystemLibrary.Delay` (* (`KismetMathLibrary.RandomFloat`) (`self.停留時間`)))
              (goto _label_2))))))))

(event `self.CapsuleComponent.OnComponentBeginOverlap`
  (params (OverlappedComponent :type "PrimitiveComponent Object Reference") (OtherActor :type "Actor Object Reference") (OtherComp :type "PrimitiveComponent Object Reference") (OtherBodyIndex :type Integer) (bFromSweep :type Boolean) (SweepResult :type "HitResult Structure (by ref)"))
  (bind `_遊戲模式` (`self.遊戲模式`))
  ;[1 0 0] 怪物受傷與死亡
  (bind `_asbp_子彈` (cast `/Game/BP/BP_子彈` OtherActor))
  (bind `_是否死亡` (`self.受傷` (`/Game/BP/BP_子彈.目前武器傷害` `_asbp_子彈`)))
  (if `_是否死亡`
    (set `/Game/BP/BP_遊戲模式.擊殺怪物數量` (+ (`/Game/BP/BP_遊戲模式.擊殺怪物數量` `_遊戲模式`) 1) `_遊戲模式`)
    (`KismetSystemLibrary.Delay` 0.8)
    (`self.K2_DestroyActor`)
    (else
      (goto _label))))

(event `self.ReceiveBeginPlay`
  (`|ExecutionSequence`
    (:`then_0`
      (goto _label_2))
    (:`then_1`
      ;[0.9287 1 0.2215] 取得遊戲模式
      (bind `_asbp_遊戲模式` (cast `/Game/BP/BP_遊戲模式` (`GameplayStatics.GetGameMode`)))
      (set `self.遊戲模式` `_asbp_遊戲模式`))
    (:`then_2`
      ;[0.5871 0.5667 1] 忽略碰撞
      (`PrimitiveComponent.IgnoreComponentWhenMoving` (`self.CapsuleComponent`) (`self.攻擊區域`) false))
    (:`then_3`
      ;[1 1 1] 取得玩家資訊
      (bind `_asbp_玩家控制` (cast `/Game/BP/BP_玩家控制` (`GameplayStatics.GetPlayerCharacter` 0)))
      (set `self.玩家控制` `_asbp_玩家控制`))))

(event `self.攻擊區域.OnComponentBeginOverlap`
  (params (OverlappedComponent :type "PrimitiveComponent Object Reference") (OtherActor :type "Actor Object Reference") (OtherComp :type "PrimitiveComponent Object Reference") (OtherBodyIndex :type Integer) (bFromSweep :type Boolean) (SweepResult :type "HitResult Structure (by ref)"))
  ;[0.5286 0.6464 1] 攻擊區域判定與傳送傷害
  (bind `_asbp_玩家控制` (cast `/Game/BP/BP_玩家控制` OtherActor))
  (`/Game/BP/BP_玩家控制.受傷` `_asbp_玩家控制` (`self.怪物攻擊力`)))

(fn `UserConstructionScript`)

(fn `受傷`
  (params (`接收傷害` :type "Float (double-precision)"))
  (returns (`是否死亡` :type Boolean))
  ;[1 0.4908 0.2785] 受傷
  (bind _output_get (set `self.血量` (- (`self.血量`) `接收傷害`)))
  (if (<= _output_get 0.0)
    ;[0 1 0.9103] 死亡
    (`PrimitiveComponent.SetSimulatePhysics` (`self.Mesh`) true) ; 模擬布偶物理效果
    (`PrimitiveComponent.SetCollisionEnabled` (`self.CapsuleComponent`) "NoCollision") ; 設定碰撞啟動 : 關閉效能碰撞避免產先太大效果
    (return true)
    (else
      (return false))))