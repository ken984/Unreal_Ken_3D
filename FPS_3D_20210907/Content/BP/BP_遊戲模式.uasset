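; Game mode Blueprint that runs a minute-and-second countdown and pauses the game when time runs out.
; On BeginPlay it counts the actors tagged "怪物" (monster) and stores the total as the required kill count, which this graph does not otherwise use.
; Tick feeds a one-second Delay that throttles the countdown, decrementing seconds, borrowing from minutes, and clamping at zero before pausing.
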(event `self.ReceiveBeginPlay`
  ;[0.9457 0.4405 1] 取得地圖上怪物數量
  (bind _outactors (`GameplayStatics.GetAllActorsWithTag` "怪物"))
  (set `self.需要擊殺怪物數量` (`KismetArrayLibrary.Array_Length` _outactors)))

(event `self.ReceiveTick`
  (params (DeltaSeconds :type "Float (single-precision)"))
  ;[1 0.1823 0.1823] 倒數系統
  ;;[1 1 1] 每秒秒數-1
  (`KismetSystemLibrary.Delay` 1.0) ; 延遲 : 等待所設定的時間在做下一個節點
  (bind _output_get (set `self.秒` (- (`self.秒`) 1)))
  ;;[1 1 1] 當秒數<0 重新設定秒數為59
  (if (< _output_get 0)
    (set `self.秒` 59)
    ;;[1 1 1] 當分>0 分-1
    (if (> (`self.分`) 0)
      (set `self.分` (- (`self.分`) 1))
      (else
        ;;[1 1 1] 當分<0, 秒等於59  將秒設為0  結束遊戲
        (if (== (`self.秒`) 59)
          (set `self.秒` 0)
          (`GameplayStatics.SetGamePaused` true))))))

(fn `UserConstructionScript`)