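; BP_武器 is a weapon Blueprint that handles firing, magazine reloading and reserve ammo.
; Holding the 開槍 input loops on a Delay while rounds remain, spawning BP_子彈 at the 子彈插槽 socket with a muzzle particle and passing it the weapon damage.
; 換彈夾 tops up the magazine from reserve, limited to what is left.
; 補充子彈 adds one magazine to reserve, clamped to the maximum.
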(event `InputAction|開槍`
  (params (Key :type "Key Structure"))
  ;[1 1 1] 開槍功能
  (:`Pressed`
    (set `self.開槍中` true)
    (if (and (> (`self.目前子彈數量`) 0) (`self.開槍中`)) :!label _label
      (bind _returnvalue (`|SpawnActorFromClass` "/Game/BP/BP_子彈.BP_子彈_C" (`SceneComponent.GetSocketTransform` (`self.武器`) "子彈插槽" "RTS_World") "Undefined" "OverrideRootScale" null null)) ; 生成子彈藍圖
      (set `/Game/BP/BP_子彈.目前武器傷害` (`self.武器傷害`) _returnvalue) ; 將武器傷害傳給子彈
      (`GameplayStatics.SpawnEmitterAtLocation` "/Game/InfinityBladeEffects/Effects/FX_Skill_Leap/P_Skill_Leap_Base_Charge_Weapon.P_Skill_Leap_Base_Charge_Weapon" (`SceneComponent.GetSocketLocation` (`self.武器`) "子彈插槽") (struct) (0.1 0.1 0.1)) ; 生成粒子在指定座標上
      (set `self.目前子彈數量` (- (`self.目前子彈數量`) 1)) ; 開槍後子彈-1
      (`KismetSystemLibrary.Delay` (`self.開槍間隔`))
      (goto _label)))
  (:`Released`
    (set `self.開槍中` false)))

(event `換彈夾`
  ;[1 1 1] 計算要補充幾顆子彈
  (set `self.要補充` (- (`self.彈夾`) (`self.目前子彈數量`))) ; 計算要補充的子彈數量 EX:\n目前10 彈夾30 所以要補充20
  ;[1 1 1] 判斷總數是否>=要補充數量
  (if (not (>= (`self.子彈總數`) (`self.要補充`)))
    ;[1 1 1] 總數<要補充數量
    (set `self.要補充` (`self.子彈總數`)))
  ;[1 1 1] 目前子彈以及總數更新
  (set `self.目前子彈數量` (+ (`self.目前子彈數量`) (`self.要補充`))) ; 補充子彈數量 \nEX : 目前10 要補充為20 補充後 目前為30
  (set `self.子彈總數` (- (`self.子彈總數`) (`self.要補充`))) ; 扣除子彈總數\nEX: 總數為20 要補充20 補充後總數為0.
)

(event `補充子彈`
  ;[1 1 1] 補充子彈
  (bind _output_get (set `self.子彈總數` (+ (`self.子彈總數`) (`self.彈夾`)))) ; 子彈總數+彈夾
  (set `self.子彈總數` (`KismetMathLibrary.Clamp` _output_get 0 (`self.子彈上限`))))

(fn `UserConstructionScript`)